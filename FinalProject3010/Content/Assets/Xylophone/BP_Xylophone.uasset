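; Xylophone actor whose key components play a sound when a Vehicle-tagged actor overlaps them.
; Each key has its own overlap handler with a DoOnce that resets after a short delay to limit retriggering.
; All keys currently play the same Collapse01 sound at their location; A3 checks the xylophone's own tag instead of the overlapping actor's.
; A data-driven PlayXylophoneNote function and SoundMap setup are unfinished and unused.
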(event OnComponentBeginOverlap(B1)
  (params (OverlappedComponent :type Primitive%20Component%20Object%20Reference) (OtherActor :type Actor%20Object%20Reference) (OtherComp :type Primitive%20Component%20Object%20Reference) (OtherBodyIndex :type Integer) (bFromSweep :type Boolean) (SweepResult :type Hit%20Result%20Structure%20%28by%20ref%29))
  (if (Actor|ActorHasTag OtherActor "Vehicle")
    (Utilities|FlowControl|DoOnce false :!label _label
      (:Completed
        (Audio|PlaySoundatLocation "/Game/PreloadedAssets(DontUse)/StarterContent/Audio/Collapse01.Collapse01" (Transformation|GetSocketLocation (Variables|Default|GetB1) "None") "0, 0, 0" 1.0 1.0 0.0 0 0 0 0)
        (Utilities|FlowControl|Delay 0.2)
        (goto _label Reset)))))

(event OnComponentBeginOverlap(C1)
  (params (OverlappedComponent :type Primitive%20Component%20Object%20Reference) (OtherActor :type Actor%20Object%20Reference) (OtherComp :type Primitive%20Component%20Object%20Reference) (OtherBodyIndex :type Integer) (bFromSweep :type Boolean) (SweepResult :type Hit%20Result%20Structure%20%28by%20ref%29))
  (if (Actor|ActorHasTag OtherActor "Vehicle")
    (Utilities|FlowControl|DoOnce false :!label _label
      (:Completed
        (Audio|PlaySoundatLocation "/Game/PreloadedAssets(DontUse)/StarterContent/Audio/Collapse01.Collapse01" (Transformation|GetSocketLocation (Variables|Default|GetC1) "None") "0, 0, 0" 1.0 1.0 0.0 0 0 0 0)
        (Utilities|FlowControl|Delay 0.2)
        (goto _label Reset)))))

(event OnComponentBeginOverlap(D1)
  (params (OverlappedComponent :type Primitive%20Component%20Object%20Reference) (OtherActor :type Actor%20Object%20Reference) (OtherComp :type Primitive%20Component%20Object%20Reference) (OtherBodyIndex :type Integer) (bFromSweep :type Boolean) (SweepResult :type Hit%20Result%20Structure%20%28by%20ref%29))
  (if (Actor|ActorHasTag OtherActor "Vehicle")
    (Utilities|FlowControl|DoOnce false :!label _label
      (:Completed
        (Audio|PlaySoundatLocation "/Game/PreloadedAssets(DontUse)/StarterContent/Audio/Collapse01.Collapse01" (Transformation|GetSocketLocation (Variables|Default|GetD1) "None") "0, 0, 0" 1.0 1.0 0.0 0 0 0 0)
        (Utilities|FlowControl|Delay 0.2)
        (goto _label Reset)))))

(event OnComponentBeginOverlap(E1)
  (params (OverlappedComponent :type Primitive%20Component%20Object%20Reference) (OtherActor :type Actor%20Object%20Reference) (OtherComp :type Primitive%20Component%20Object%20Reference) (OtherBodyIndex :type Integer) (bFromSweep :type Boolean) (SweepResult :type Hit%20Result%20Structure%20%28by%20ref%29))
  (if (Actor|ActorHasTag OtherActor "Vehicle")
    (Utilities|FlowControl|DoOnce false :!label _label
      (:Completed
        (Audio|PlaySoundatLocation "/Game/PreloadedAssets(DontUse)/StarterContent/Audio/Collapse01.Collapse01" (Transformation|GetSocketLocation (Variables|Default|GetE1) "None") "0, 0, 0" 1.0 1.0 0.0 0 0 0 0)
        (Utilities|FlowControl|Delay 0.2)
        (goto _label Reset)))))

(event OnComponentBeginOverlap(F1)
  (params (OverlappedComponent :type Primitive%20Component%20Object%20Reference) (OtherActor :type Actor%20Object%20Reference) (OtherComp :type Primitive%20Component%20Object%20Reference) (OtherBodyIndex :type Integer) (bFromSweep :type Boolean) (SweepResult :type Hit%20Result%20Structure%20%28by%20ref%29))
  (if (Actor|ActorHasTag OtherActor "Vehicle")
    (Utilities|FlowControl|DoOnce false :!label _label
      (:Completed
        (Audio|PlaySoundatLocation "/Game/PreloadedAssets(DontUse)/StarterContent/Audio/Collapse01.Collapse01" (Transformation|GetSocketLocation (Variables|Default|GetF1) "None") "0, 0, 0" 1.0 1.0 0.0 0 0 0 0)
        (Utilities|FlowControl|Delay 0.2)
        (goto _label Reset)))))

(event OnComponentBeginOverlap(G2)
  (params (OverlappedComponent :type Primitive%20Component%20Object%20Reference) (OtherActor :type Actor%20Object%20Reference) (OtherComp :type Primitive%20Component%20Object%20Reference) (OtherBodyIndex :type Integer) (bFromSweep :type Boolean) (SweepResult :type Hit%20Result%20Structure%20%28by%20ref%29))
  (if (Actor|ActorHasTag OtherActor "Vehicle")
    (Utilities|FlowControl|DoOnce false :!label _label
      (:Completed
        (Audio|PlaySoundatLocation "/Game/PreloadedAssets(DontUse)/StarterContent/Audio/Collapse01.Collapse01" (Transformation|GetSocketLocation (Variables|Default|GetG2) "None") "0, 0, 0" 1.0 1.0 0.0 0 0 0 0)
        (Utilities|FlowControl|Delay 0.2)
        (goto _label Reset)))))

(event OnComponentBeginOverlap(A2)
  (params (OverlappedComponent :type Primitive%20Component%20Object%20Reference) (OtherActor :type Actor%20Object%20Reference) (OtherComp :type Primitive%20Component%20Object%20Reference) (OtherBodyIndex :type Integer) (bFromSweep :type Boolean) (SweepResult :type Hit%20Result%20Structure%20%28by%20ref%29))
  (if (Actor|ActorHasTag OtherActor "Vehicle")
    (Utilities|FlowControl|DoOnce false :!label _label
      (:Completed
        (Audio|PlaySoundatLocation "/Game/PreloadedAssets(DontUse)/StarterContent/Audio/Collapse01.Collapse01" (Transformation|GetSocketLocation (Variables|Default|GetA2) "None") "0, 0, 0" 1.0 1.0 0.0 0 0 0 0)
        (Utilities|FlowControl|Delay 0.2)
        (goto _label Reset)))))

(event OnComponentBeginOverlap(B2)
  (params (OverlappedComponent :type Primitive%20Component%20Object%20Reference) (OtherActor :type Actor%20Object%20Reference) (OtherComp :type Primitive%20Component%20Object%20Reference) (OtherBodyIndex :type Integer) (bFromSweep :type Boolean) (SweepResult :type Hit%20Result%20Structure%20%28by%20ref%29))
  (if (Actor|ActorHasTag OtherActor "Vehicle")
    (Utilities|FlowControl|DoOnce false :!label _label
      (:Completed
        (Audio|PlaySoundatLocation "/Game/PreloadedAssets(DontUse)/StarterContent/Audio/Collapse01.Collapse01" (Transformation|GetSocketLocation (Variables|Default|GetB2) "None") "0, 0, 0" 1.0 1.0 0.0 0 0 0 0)
        (Utilities|FlowControl|Delay 0.2)
        (goto _label Reset)))))

(event OnComponentBeginOverlap(C2)
  (params (OverlappedComponent :type Primitive%20Component%20Object%20Reference) (OtherActor :type Actor%20Object%20Reference) (OtherComp :type Primitive%20Component%20Object%20Reference) (OtherBodyIndex :type Integer) (bFromSweep :type Boolean) (SweepResult :type Hit%20Result%20Structure%20%28by%20ref%29))
  (if (Actor|ActorHasTag OtherActor "Vehicle")
    (Utilities|FlowControl|DoOnce false :!label _label
      (:Completed
        (Audio|PlaySoundatLocation "/Game/PreloadedAssets(DontUse)/StarterContent/Audio/Collapse01.Collapse01" (Transformation|GetSocketLocation (Variables|Default|GetC2) "None") "0, 0, 0" 1.0 1.0 0.0 0 0 0 0)
        (Utilities|FlowControl|Delay 0.2)
        (goto _label Reset)))))

(event OnComponentBeginOverlap(D2)
  (params (OverlappedComponent :type Primitive%20Component%20Object%20Reference) (OtherActor :type Actor%20Object%20Reference) (OtherComp :type Primitive%20Component%20Object%20Reference) (OtherBodyIndex :type Integer) (bFromSweep :type Boolean) (SweepResult :type Hit%20Result%20Structure%20%28by%20ref%29))
  (if (Actor|ActorHasTag OtherActor "Vehicle")
    (Utilities|FlowControl|DoOnce false :!label _label
      (:Completed
        (Audio|PlaySoundatLocation "/Game/PreloadedAssets(DontUse)/StarterContent/Audio/Collapse01.Collapse01" (Transformation|GetSocketLocation (Variables|Default|GetD2) "None") "0, 0, 0" 1.0 1.0 0.0 0 0 0 0)
        (Utilities|FlowControl|Delay 0.2)
        (goto _label Reset)))))

(event OnComponentBeginOverlap(E2)
  (params (OverlappedComponent :type Primitive%20Component%20Object%20Reference) (OtherActor :type Actor%20Object%20Reference) (OtherComp :type Primitive%20Component%20Object%20Reference) (OtherBodyIndex :type Integer) (bFromSweep :type Boolean) (SweepResult :type Hit%20Result%20Structure%20%28by%20ref%29))
  (if (Actor|ActorHasTag OtherActor "Vehicle")
    (Utilities|FlowControl|DoOnce false :!label _label
      (:Completed
        (Audio|PlaySoundatLocation "/Game/PreloadedAssets(DontUse)/StarterContent/Audio/Collapse01.Collapse01" (Transformation|GetSocketLocation (Variables|Default|GetE2) "None") "0, 0, 0" 1.0 1.0 0.0 0 0 0 0)
        (Utilities|FlowControl|Delay 0.2)
        (goto _label Reset)))))

(event OnComponentBeginOverlap(F2)
  (params (OverlappedComponent :type Primitive%20Component%20Object%20Reference) (OtherActor :type Actor%20Object%20Reference) (OtherComp :type Primitive%20Component%20Object%20Reference) (OtherBodyIndex :type Integer) (bFromSweep :type Boolean) (SweepResult :type Hit%20Result%20Structure%20%28by%20ref%29))
  (if (Actor|ActorHasTag OtherActor "Vehicle")
    (Utilities|FlowControl|DoOnce false :!label _label
      (:Completed
        (Audio|PlaySoundatLocation "/Game/PreloadedAssets(DontUse)/StarterContent/Audio/Collapse01.Collapse01" (Transformation|GetSocketLocation (Variables|Default|GetF2) "None") "0, 0, 0" 1.0 1.0 0.0 0 0 0 0)
        (Utilities|FlowControl|Delay 0.2)
        (goto _label Reset)))))

(event OnComponentBeginOverlap(G3)
  (params (OverlappedComponent :type Primitive%20Component%20Object%20Reference) (OtherActor :type Actor%20Object%20Reference) (OtherComp :type Primitive%20Component%20Object%20Reference) (OtherBodyIndex :type Integer) (bFromSweep :type Boolean) (SweepResult :type Hit%20Result%20Structure%20%28by%20ref%29))
  (if (Actor|ActorHasTag OtherActor "Vehicle")
    (Utilities|FlowControl|DoOnce false :!label _label
      (:Completed
        (Audio|PlaySoundatLocation "/Game/PreloadedAssets(DontUse)/StarterContent/Audio/Collapse01.Collapse01" (Transformation|GetSocketLocation (Variables|Default|GetG3) "None") "0, 0, 0" 1.0 1.0 0.0 0 0 0 0)
        (Utilities|FlowControl|Delay 0.2)
        (goto _label Reset)))))

(event OnComponentBeginOverlap(A3)
  (params (OverlappedComponent :type Primitive%20Component%20Object%20Reference) (OtherActor :type Actor%20Object%20Reference) (OtherComp :type Primitive%20Component%20Object%20Reference) (OtherBodyIndex :type Integer) (bFromSweep :type Boolean) (SweepResult :type Hit%20Result%20Structure%20%28by%20ref%29))
  (if (Actor|ActorHasTag "Vehicle")
    (Utilities|FlowControl|DoOnce false :!label _label
      (:Completed
        (Audio|PlaySoundatLocation "/Game/PreloadedAssets(DontUse)/StarterContent/Audio/Collapse01.Collapse01" (Transformation|GetSocketLocation (Variables|Default|GetA3) "None") "0, 0, 0" 1.0 1.0 0.0 0 0 0 0)
        (Utilities|FlowControl|Delay 0.2)
        (goto _label Reset)))))

(event OnComponentBeginOverlap(A1)
  (params (OverlappedComponent :type Primitive%20Component%20Object%20Reference) (OtherActor :type Actor%20Object%20Reference) (OtherComp :type Primitive%20Component%20Object%20Reference) (OtherBodyIndex :type Integer) (bFromSweep :type Boolean) (SweepResult :type Hit%20Result%20Structure%20%28by%20ref%29))
  (if (Actor|ActorHasTag OtherActor "Vehicle")
    (Utilities|FlowControl|DoOnce false :!label _label
      (:Completed
        (Audio|PlaySoundatLocation "/Game/PreloadedAssets(DontUse)/StarterContent/Audio/Collapse01.Collapse01" (Transformation|GetSocketLocation (Variables|Default|GetA1) "None") "0, 0, 0" 1.0 1.0 0.0 0 0 0 0)
        (Utilities|FlowControl|Delay 0.2)
        (goto _label Reset)))))

(event OnComponentBeginOverlap(G1)
  (params (OverlappedComponent :type Primitive%20Component%20Object%20Reference) (OtherActor :type Actor%20Object%20Reference) (OtherComp :type Primitive%20Component%20Object%20Reference) (OtherBodyIndex :type Integer) (bFromSweep :type Boolean) (SweepResult :type Hit%20Result%20Structure%20%28by%20ref%29))
  (if (Actor|ActorHasTag OtherActor "Vehicle")
    (Utilities|FlowControl|DoOnce false :!label _label
      (:Completed
        (Audio|PlaySoundatLocation "/Game/PreloadedAssets(DontUse)/StarterContent/Audio/Collapse01.Collapse01" (Transformation|GetSocketLocation (Variables|Default|GetG1) "None") "0, 0, 0" 1.0 1.0 0.0 0 0 0 0)
        (Utilities|FlowControl|Delay 0.2)
        (goto _label Reset)))))

(event EventBeginPlay)

(fn ConstructionScript)

(fn PlayXylophoneNote
  (params (keyName :type String) (OtherActor :type Actor%20Object%20Reference) (keyLocation :type Vector))
  (if (Actor|ActorHasTag OtherActor "Vehicle")
    (Utilities|FlowControl|DoOnce false)))