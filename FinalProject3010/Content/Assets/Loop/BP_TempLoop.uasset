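; BP_TempLoop is a loop actor that stages a brief, one-time camera change for a sports car.
; OnInteract prints a debug message and stores the interacting vehicle as SportsCar.
; The first overlap of FirstCollisionBox with a valid SportsCar attaches its FrontCamera to CameraPositionArrow, flips the camera, then flips it back two seconds later.
; The overlap does not check which actor entered, and the camera is never reattached here.
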(event OnComponentBeginOverlap(FirstCollisionBox)
  (params (OverlappedComponent :type Primitive%20Component%20Object%20Reference) (OtherActor :type Actor%20Object%20Reference) (OtherComp :type Primitive%20Component%20Object%20Reference) (OtherBodyIndex :type Integer) (bFromSweep :type Boolean) (SweepResult :type Hit%20Result%20Structure%20%28by%20ref%29))
  (bind _sportscar (Variables|Default|GetSportsCar)
    (:then
      (Utilities|FlowControl|DoOnce false
        (:Completed
          (Transformation|AttachComponentToComponent (Variables|/Game/VehicleTemplate/Blueprints/VehicleAdvPawn.VehicleAdvPawn_C|GetFrontCamera _sportscar) (Variables|Default|GetCameraPosition%28Arrow%29) "None" "KeepRelative" "KeepRelative" "KeepRelative" true)
          (Default|FlipCamera _sportscar)
          (Utilities|FlowControl|Delay 2.0)
          (Default|FlipCamera _sportscar))))
    (:else)))

(event EventBeginPlay)

(event Collision|EventActorBeginOverlap
  (params (OtherActor :type Actor%20Object%20Reference)))

(event EventTick
  (params (DeltaSeconds :type Float%20%28single-precision%29)))

(event EventOnInteract
  (params (Vehicle :type Sports%20Car%20Pawn%20Object%20Reference))
  (Development|PrintString "interacted")
  (Variables|Default|SetSportsCar Vehicle))

(fn ConstructionScript)